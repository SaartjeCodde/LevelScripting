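; Main menu actor built from clickable components for new game, level select among three levels, and quit.
; Clicks play a sound and flip submenus through ToggleVisibility, so state depends on starting visibility; only Back explicitly hides the level buttons.
; Hover events swap selected and unselected materials by creating a new dynamic material instance each time.
; Level and quit buttons pause briefly before opening a level or exiting.
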(event OnClicked(Play)
  (params (TouchedComponent :type Primitive%20Component%20Object%20Reference))
  ;[1 1 1] Visibility toggles
  (Audio|PlaySoundatLocation "/Game/Sound/MenuClick.MenuClick" "0, 0, 0")
  (Rendering|ToggleVisibility (Variables|Default|GetBack) false)
  (Rendering|ToggleVisibility (Variables|Default|GetPlay) false))

(event OnBeginCursorOver(Play)
  (params (TouchedComponent :type Primitive%20Component%20Object%20Reference))
  ;[1 1 1] Changing material when selected or not
  (Rendering|Material|CreateDynamicMaterialInstance (Variables|Default|GetPlay) 0 (Variables|Default|GetMaterialSelected) :!class /Script/Engine.PrimitiveComponent))

(event OnEndCursorOver(Play)
  (params (TouchedComponent :type Primitive%20Component%20Object%20Reference))
  ;[1 1 1] Changing material when selected or not
  (Rendering|Material|CreateDynamicMaterialInstance (Variables|Default|GetPlay) 0 (Variables|Default|GetMaterialNotSelected) :!class /Script/Engine.PrimitiveComponent))

(event OnEndCursorOver(Back)
  (params (TouchedComponent :type Primitive%20Component%20Object%20Reference))
  ;[1 1 1] Changing material when selected or not
  (Rendering|Material|CreateDynamicMaterialInstance (Variables|Default|GetBack) 0 (Variables|Default|GetMaterialNotSelected) :!class /Script/Engine.PrimitiveComponent))

(event OnBeginCursorOver(Back)
  (params (TouchedComponent :type Primitive%20Component%20Object%20Reference))
  ;[1 1 1] Changing material when selected or not
  (Rendering|Material|CreateDynamicMaterialInstance (Variables|Default|GetBack) 0 (Variables|Default|GetMaterialSelected) :!class /Script/Engine.PrimitiveComponent))

(event OnBeginCursorOver(Level1)
  (params (TouchedComponent :type Primitive%20Component%20Object%20Reference))
  ;[1 1 1] Changing material when selected or not
  (Rendering|Material|CreateDynamicMaterialInstance (Variables|Default|GetLevel1) 0 (Variables|Default|GetMaterialSelected) :!class /Script/Engine.PrimitiveComponent))

(event OnEndCursorOver(Level1)
  (params (TouchedComponent :type Primitive%20Component%20Object%20Reference))
  ;[1 1 1] Changing material when selected or not
  (Rendering|Material|CreateDynamicMaterialInstance (Variables|Default|GetLevel1) 0 (Variables|Default|GetMaterialNotSelected) :!class /Script/Engine.PrimitiveComponent))

(event OnBeginCursorOver(Level2)
  (params (TouchedComponent :type Primitive%20Component%20Object%20Reference))
  ;[1 1 1] Changing material when selected or not
  (Rendering|Material|CreateDynamicMaterialInstance (Variables|Default|GetLevel2) 0 (Variables|Default|GetMaterialSelected) :!class /Script/Engine.PrimitiveComponent))

(event OnEndCursorOver(Level2)
  (params (TouchedComponent :type Primitive%20Component%20Object%20Reference))
  ;[1 1 1] Changing material when selected or not
  (Rendering|Material|CreateDynamicMaterialInstance (Variables|Default|GetLevel2) 0 (Variables|Default|GetMaterialNotSelected) :!class /Script/Engine.PrimitiveComponent))

(event OnBeginCursorOver(Level3)
  (params (TouchedComponent :type Primitive%20Component%20Object%20Reference))
  ;[1 1 1] Changing material when selected or not
  (Rendering|Material|CreateDynamicMaterialInstance (Variables|Default|GetLevel3) 0 (Variables|Default|GetMaterialSelected) :!class /Script/Engine.PrimitiveComponent))

(event OnEndCursorOver(Level3)
  (params (TouchedComponent :type Primitive%20Component%20Object%20Reference))
  ;[1 1 1] Changing material when selected or not
  (Rendering|Material|CreateDynamicMaterialInstance (Variables|Default|GetLevel3) 0 (Variables|Default|GetMaterialNotSelected) :!class /Script/Engine.PrimitiveComponent))

(event OnEndCursorOver(LevelSelect)
  (params (TouchedComponent :type Primitive%20Component%20Object%20Reference))
  ;[1 1 1] Changing material when selected or not
  (Rendering|Material|CreateDynamicMaterialInstance (Variables|Default|GetLevelSelect) 0 (Variables|Default|GetMaterialNotSelected) :!class /Script/Engine.PrimitiveComponent))

(event OnBeginCursorOver(LevelSelect)
  (params (TouchedComponent :type Primitive%20Component%20Object%20Reference))
  ;[1 1 1] Changing material when selected or not
  (Rendering|Material|CreateDynamicMaterialInstance (Variables|Default|GetLevelSelect) 0 (Variables|Default|GetMaterialSelected) :!class /Script/Engine.PrimitiveComponent))

(event OnEndCursorOver(Quit)
  (params (TouchedComponent :type Primitive%20Component%20Object%20Reference))
  ;[1 1 1] Changing material when selected or not
  (Rendering|Material|CreateDynamicMaterialInstance (Variables|Default|GetQuit) 0 (Variables|Default|GetMaterialNotSelected) :!class /Script/Engine.PrimitiveComponent))

(event OnBeginCursorOver(Quit)
  (params (TouchedComponent :type Primitive%20Component%20Object%20Reference))
  ;[1 1 1] Changing material when selected or not
  (Rendering|Material|CreateDynamicMaterialInstance (Variables|Default|GetQuit) 0 (Variables|Default|GetMaterialSelected) :!class /Script/Engine.PrimitiveComponent))

(event OnEndCursorOver(NewGame)
  (params (TouchedComponent :type Primitive%20Component%20Object%20Reference))
  ;[1 1 1] Changing material when selected or not
  (Rendering|Material|CreateDynamicMaterialInstance (Variables|Default|GetNewGame) 0 (Variables|Default|GetMaterialNotSelected) :!class /Script/Engine.PrimitiveComponent))

(event OnBeginCursorOver(NewGame)
  (params (TouchedComponent :type Primitive%20Component%20Object%20Reference))
  ;[1 1 1] Changing material when selected or not
  (Rendering|Material|CreateDynamicMaterialInstance (Variables|Default|GetNewGame) 0 (Variables|Default|GetMaterialSelected) :!class /Script/Engine.PrimitiveComponent))

(event OnClicked(Quit)
  (params (TouchedComponent :type Primitive%20Component%20Object%20Reference))
  ;[1 1 1] OnClicked events
  (Audio|PlaySoundatLocation "/Game/Sound/MenuClick.MenuClick" "0, 0, 0")
  (Utilities|FlowControl|Delay 0.2)
  (Game|QuitGame 0 "Quit"))

(event OnClicked(LevelSelect)
  (params (TouchedComponent :type Primitive%20Component%20Object%20Reference))
  ;[1 1 1] Visibility toggles
  (Audio|PlaySoundatLocation "/Game/Sound/MenuClick.MenuClick" "0, 0, 0")
  (Rendering|ToggleVisibility (Variables|Default|GetLevel3) false))

(event OnClicked(Back)
  (params (TouchedComponent :type Primitive%20Component%20Object%20Reference))
  ;[1 1 1] Visibility toggles
  (Audio|PlaySoundatLocation "/Game/Sound/MenuClick.MenuClick" "0, 0, 0")
  (Rendering|SetVisibility (Variables|Default|GetLevel3) false false)
  (Rendering|ToggleVisibility (Variables|Default|GetNewGame) false)
  (Rendering|ToggleVisibility (Variables|Default|GetPlay) false))

(event OnClicked(Level1)
  (params (TouchedComponent :type Primitive%20Component%20Object%20Reference))
  ;[1 1 1] OnClicked events
  (Audio|PlaySoundatLocation "/Game/Sound/MenuClick.MenuClick" "0, 0, 0")
  (Utilities|FlowControl|Delay 0.2)
  (Game|OpenLevel(byName) "Level_01"))

(event OnClicked(Level2)
  (params (TouchedComponent :type Primitive%20Component%20Object%20Reference))
  ;[1 1 1] OnClicked events
  (Audio|PlaySoundatLocation "/Game/Sound/MenuClick.MenuClick" "0, 0, 0")
  (Utilities|FlowControl|Delay 0.2)
  (Game|OpenLevel(byName) "Level_02"))

(event OnClicked(Level3)
  (params (TouchedComponent :type Primitive%20Component%20Object%20Reference))
  ;[1 1 1] OnClicked events
  (Audio|PlaySoundatLocation "/Game/Sound/MenuClick.MenuClick" "0, 0, 0")
  (Utilities|FlowControl|Delay 0.2)
  (Game|OpenLevel(byName) "Level_03"))

(event OnClicked(NewGame)
  (params (TouchedComponent :type Primitive%20Component%20Object%20Reference))
  ;[1 1 1] OnClicked events
  (Audio|PlaySoundatLocation "/Game/Sound/MenuClick.MenuClick" "0, 0, 0")
  (Utilities|FlowControl|Delay 0.2)
  (Game|OpenLevel(byName) "Level_01"))

(event EventBeginPlay
  ;[1 1 1] Visibility toggles
  (Rendering|ToggleVisibility (Variables|Default|GetNewGame) false))

(fn ConstructionScript)