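; KnightCharacter is the player pawn for a side-scrolling knight game, moving along one world axis and jumping with a sound.
; On BeginPlay it resets health, stores its spawn transform in KnightSideScrollerMode and creates the HUD.
; Tick destroys it when health runs out, and P pauses the game with a pause menu.
; Functions track keys, diamonds and fixed-step damage, while an event restores default jump velocity.
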(event Custom|Reset%20Jump%20Z%20Vel
  (Variables|/Script/Engine.CharacterMovementComponent|SetJumpZVelocity (Variables|Character|GetCharacterMovement) 1e+03))

(event EventBeginPlay
  ;[1 1 1] (re)spawn
  (Variables|Default|SetHealth 1e+02)
  (bind _asknight_side_scroller_mode (Utilities|Casting|CastToKnightSideScrollerMode (Game|GetGameMode)))
  (Variables|/Game/Blueprints/Game/KnightSideScrollerMode.KnightSideScrollerMode_C|SetSpawn%20Transform _asknight_side_scroller_mode (Transformation|GetActorTransform))
  (bind _returnvalue (UserInterface|CreateWidget "/Game/Blueprints/Game/KnightGameHUD.KnightGameHUD_C"))
  (bind _output_get (Variables|Default|SetGame%20HUD%20Widget _returnvalue))
  (UserInterface|Viewport|AddtoViewport _output_get 0))

(event EventEndPlay
  (params (EndPlayReason :type EEndPlayReason%20Enum :default "ActorDestroyed"))
  ;[1 1 1] Pause
  (Widget|RemovefromParent (Variables|Default|GetGame%20HUD%20Widget)))

(event EventTick
  (params (DeltaSeconds :type Float%20%28single-precision%29))
  ;[1 1 1] Kill
  (if (<= (Variables|Default|GetHealth) 0.0)
    (Widget|RemovefromParent (Variables|Default|GetGame%20HUD%20Widget))
    (Actor|DestroyActor)))

(event Input|ActionEvents|InputActionJump
  ;[1 1 1] Movement
  (:Pressed
    (Character|Jump)
    (Audio|PlaySoundatLocation "/Game/Sound/Jump.Jump" "0, 0, 0"))
  (:Released
    (Character|StopJumping)))

(event Input|AxisEvents|InputAxisMoveRight
  (params (AxisValue :type Float%20%28single-precision%29))
  ;[1 1 1] Movement
  (Pawn|Input|AddMovementInput "0,-1.000000, 0" AxisValue false))

(event Input|KeyboardEvents|P
  ;[1 1 1] Pause
  (:Pressed
    (Game|SetGamePaused true)
    (bind _returnvalue (UserInterface|CreateWidget "/Game/Blueprints/Game/PauseMenu.PauseMenu_C"))
    (bind _output_get (Variables|Default|SetPause%20Menu%20Widget _returnvalue))
    (UserInterface|Viewport|AddtoViewport _output_get 0)))

(fn ConstructionScript)

(fn PlayerHoldsKey
  (bind _output_get (Variables|Default|SetPlayerHasKey true))
  (Variables|Default|SetAmountOfKeys (+ (Variables|Default|GetAmountOfKeys) 1.0))
  (return _output_get))

(fn PickedUpDiamond
  (Variables|Default|SetAmountOfDiamonds (+ (Variables|Default|GetAmountOfDiamonds) 1.0)))

(fn SetHealth
  (bind _output_get (Variables|Default|SetHealth (- (Variables|Default|GetHealth) 25.0)))
  (return _output_get))