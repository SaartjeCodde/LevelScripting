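; AI_Character is a critter enemy that hurts the player's knight and can be killed through a separate trigger volume.
; An overlap on HitBox casts the player pawn to KnightCharacter, calls SetHealth on it and plays a hit sound.
; An overlap on KillBox spawns a particle effect just above the critter, plays a death sound and destroys the actor.
; Neither overlap checks which actor entered the box.
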(event OnComponentBeginOverlap(HitBox)
  (params (OtherActor :type Actor%20Object%20Reference) (OtherComp :type Primitive%20Component%20Object%20Reference) (OtherBodyIndex :type Integer) (bFromSweep :type Boolean) (SweepResult :type Hit%20Result%20Structure%20%28by%20ref%29))
  ;[1 1 1] Hit player
  (bind _asknight_character (Utilities|Casting|CastToKnightCharacter (Game|Player|GetPlayerPawn 0)))
  (Default|SetHealth _asknight_character)
  (Audio|PlaySoundatLocation "/Game/Sound/SpikesOrEnemy.SpikesOrEnemy" "0, 0, 0"))

(event OnComponentBeginOverlap(KillBox)
  (params (OtherActor :type Actor%20Object%20Reference) (OtherComp :type Primitive%20Component%20Object%20Reference) (OtherBodyIndex :type Integer) (bFromSweep :type Boolean) (SweepResult :type Hit%20Result%20Structure%20%28by%20ref%29))
  (bind _returnvalue (Transformation|GetActorLocation))
  (bind (_x _y _z) (Math|Vector|BreakVector _returnvalue))
  ;[1 1 1] Kill critter
  (Effects|SpawnEmitteratLocation (Variables|Default|GetParticles) (Math|Vector|MakeVector _x _y (+ _z 5e+01)))
  (Audio|PlaySoundatLocation "/Game/Sound/EnemyKilled.EnemyKilled" "0, 0, 0")
  (Actor|DestroyActor))

(fn ConstructionScript)