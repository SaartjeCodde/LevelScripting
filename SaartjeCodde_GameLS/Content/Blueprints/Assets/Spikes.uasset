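; Spike hazard actor that damages the player's KnightCharacter and can either move on its own or shift when triggered.
; Any TriggerBox overlap plays a hit sound and calls SetHealth on the player pawn, without checking which actor overlapped.
; Two timelines lerp the Spikes component between StartPos and EndPos: MovingSpikes starts at BeginPlay if AreMovingSpikes is set, while TriggerSpikes runs on the ClearPath event.
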(event OnComponentBeginOverlap(TriggerBox)
  (params (OtherActor :type Actor%20Object%20Reference) (OtherComp :type Primitive%20Component%20Object%20Reference) (OtherBodyIndex :type Integer) (bFromSweep :type Boolean) (SweepResult :type Hit%20Result%20Structure%20%28by%20ref%29))
  ;[1 1 1] Player hit
  (Audio|PlaySoundatLocation "/Game/Sound/SpikesOrEnemy.SpikesOrEnemy" "0, 0, 0")
  (bind _asknight_character (Utilities|Casting|CastToKnightCharacter (Game|Player|GetPlayerPawn 0)))
  (Default|SetHealth _asknight_character))

(event Custom|ClearPath
  ;[1 1 1] Trigger spike
  (bind _triggerspike (Timeline|TriggerSpikes Play)
    (:Update
      (Transformation|SetRelativeLocation (Variables|Default|GetSpikes) (Math|Vector|Lerp(Vector) (Variables|Default|GetStartPos) (Variables|Default|GetEndPos) _triggerspike) false))))

(event EventBeginPlay
  ;[1 1 1] Moving spike
  (if (Variables|Default|GetAreMovingSpikes)
    (bind _moving_spikes (Timeline|Moving%20Spikes Play)
      (:Update
        (Transformation|SetRelativeLocation (Variables|Default|GetSpikes) (Math|Vector|Lerp(Vector) (Variables|Default|GetStartPos) (Variables|Default|GetEndPos) _moving_spikes) false)))))

(fn ConstructionScript)