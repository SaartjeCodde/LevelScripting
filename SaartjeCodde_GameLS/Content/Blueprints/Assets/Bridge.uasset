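; Bridge actor that slides its mesh between a start and an end position when opened or closed.
; BridgeOpen plays a timeline that lerps the mesh's relative location without sweep, and CloseBridge reverses that timeline.
; On BeginPlay it sets the mesh's first material slot to a dynamic instance of BridgeMaterial.
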(event Custom|Bridge%20Open
  ;[1 1 1] Open/close bridge
  (bind _bridge (Timeline|Bridge%20Timeline Play)
    (:Update
      (Transformation|SetRelativeLocation (Variables|Default|GetBridge) (Math|Vector|Lerp(Vector) (Variables|Default|GetBridgeStart) (Variables|Default|GetBridgeEnd) _bridge) false))))

(event Custom|Close%20Bridge
  ;[1 1 1] Open/close bridge
  (bind _bridge (Timeline|Bridge%20Timeline Reverse)
    (:Update
      (Transformation|SetRelativeLocation (Variables|Default|GetBridge) (Math|Vector|Lerp(Vector) (Variables|Default|GetBridgeStart) (Variables|Default|GetBridgeEnd) _bridge) false))))

(event EventBeginPlay
  ;[1 1 1] Change material
  (Rendering|Material|CreateDynamicMaterialInstance (Variables|Default|GetBridge) 0 (Variables|Default|GetBridgeMaterial) :!class /Script/Engine.PrimitiveComponent))

(fn ConstructionScript)