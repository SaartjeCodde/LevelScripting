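; One-shot pressure button actor that activates a floating platform, clears spikes or raises a moving platform when an actor overlaps it.
; The UsesFloatingPlatform and UsesSpikes flags select which referenced actor receives the call, with the moving platform as fallback.
; If that reference is valid, a timeline lerps the button between its start and end locations and sets IsButtonPressed, blocking further triggers.
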(event EventActorBeginOverlap
  (params (OtherActor :type Actor%20Object%20Reference))
  (bind _moving_platform (Variables|Default|GetMoving%20Platform))
  (bind _floating_platform (Variables|Default|GetFloating%20Platform))
  (bind _spikes (Variables|Default|GetSpikes))
  (if (not (Variables|Default|GetIsButtonPressed))
    (Audio|PlaySoundatLocation "/Game/Sound/ButtonOrWheel.ButtonOrWheel" "0, 0, 0")
    (if (Variables|Default|GetUsesFloatingPlatform)
      (Utilities|IsValid _floating_platform
        (:Is%20Valid
          (Default|PlatformUp _floating_platform)
          (bind _button (Timeline|Button%20Timeline Play)
            (:Update
              (Transformation|SetActorRelativeLocation (Math|Vector|Lerp(Vector) (Variables|Default|GetButtonStart) (Variables|Default|GetButtonEnd) _button))
              (Variables|Default|SetIsButtonPressed true)))))
      (elif (Variables|Default|GetUsesSpikes)
        (Utilities|IsValid _spikes
          (:Is%20Valid
            (Default|ClearPath _spikes)
            (Timeline|Button%20Timeline Play)))
        (else
          (Utilities|IsValid _moving_platform
            (:Is%20Valid
              (Default|PlatformGoUp _moving_platform)
              (Timeline|Button%20Timeline Play))))))))

(fn ConstructionScript)