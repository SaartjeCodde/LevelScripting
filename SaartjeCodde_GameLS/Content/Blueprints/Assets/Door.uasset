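; Key-locked door Blueprint that the player opens by pressing O inside its trigger box while holding a key.
; TriggerBox overlaps toggle player input; opening clears PlayerHasKey and decrements AmountOfKeys on the KnightCharacter.
; DoorOpen plays a sound at world origin and a timeline that lerps the mesh from DoorStart to DoorEnd.
; A separate TriggerPlayerInfo overlap shows a feedback widget for three seconds, guarded to appear only once.
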(event OnComponentBeginOverlap(TriggerPlayerInfo)
  (params (OtherActor :type Actor%20Object%20Reference) (OtherComp :type Primitive%20Component%20Object%20Reference) (OtherBodyIndex :type Integer) (bFromSweep :type Boolean) (SweepResult :type Hit%20Result%20Structure%20%28by%20ref%29))
  ;[1 1 1] Player feedback
  (if (not (Variables|Default|GetPlayerInfoPopped))
    (bind _returnvalue (UserInterface|CreateWidget "/Game/Blueprints/Game/PlayerFeedback_Door.PlayerFeedback_Door_C"))
    (UserInterface|Viewport|AddtoViewport _returnvalue 0)
    (Variables|Default|SetPlayerInfoPopped true)
    (Utilities|FlowControl|Delay 3.0)
    (Widget|RemovefromParent _returnvalue)))

(event OnComponentBeginOverlap(TriggerBox)
  (params (OtherActor :type Actor%20Object%20Reference) (OtherComp :type Primitive%20Component%20Object%20Reference) (OtherBodyIndex :type Integer) (bFromSweep :type Boolean) (SweepResult :type Hit%20Result%20Structure%20%28by%20ref%29))
  ;[1 1 1] Input
  (Input|EnableInput (Game|GetPlayerController 0))
  (bind _asknight_character (Utilities|Casting|CastToKnightCharacter (Game|Player|GetPlayerPawn 0))))

(event OnComponentEndOverlap(TriggerBox)
  (params (OtherActor :type Actor%20Object%20Reference) (OtherComp :type Primitive%20Component%20Object%20Reference) (OtherBodyIndex :type Integer))
  ;[1 1 1] Input
  (Input|DisableInput (Game|GetPlayerController 0)))

(event Custom|Door%20Open
  ;[1 1 1] Open door
  (Audio|PlaySoundatLocation "/Game/Sound/Door.Door" "0, 0, 0")
  (bind _door (Timeline|Door%20Timeline Play)
    (:Update
      (Transformation|SetRelativeLocation (Variables|Default|GetDoor) (Math|Vector|Lerp(Vector) (Variables|Default|GetDoorStart) (Variables|Default|GetDoorEnd) _door) false))))

(event Input|KeyboardEvents|O
  ;[1 1 1] Input
  (:Pressed
    (if (Variables|/Game/Blueprints/Player/KnightCharacter.KnightCharacter_C|GetPlayerHasKey (stale OnComponentBeginOverlap(TriggerBox) _asknight_character))
      (CallFunction|DoorOpen)
      (bind _asknight_character (Utilities|Casting|CastToKnightCharacter (Game|Player|GetPlayerPawn 0)))
      (Variables|/Game/Blueprints/Player/KnightCharacter.KnightCharacter_C|SetPlayerHasKey _asknight_character false)
      (Variables|/Game/Blueprints/Player/KnightCharacter.KnightCharacter_C|SetAmountOfKeys _asknight_character (- (Variables|/Game/Blueprints/Player/KnightCharacter.KnightCharacter_C|GetAmountOfKeys _asknight_character) 1.0)))))

(fn ConstructionScript)