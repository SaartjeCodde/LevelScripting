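; Moving platform actor that lerps its mesh's relative location between start and end points, either automatically or by trigger.
; Without IsTrigger, BeginPlay starts the MovingPlatform timeline.
; With it, each box overlap toggles PlatformDown to play or reverse a second timeline, and ending the overlap stops it mid-travel.
; BeginPlay also creates a dynamic material instance on the mesh, with no sweep used during movement.
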(event OnComponentBeginOverlap(Box)
  (params (OtherActor :type Actor%20Object%20Reference) (OtherComp :type Primitive%20Component%20Object%20Reference) (OtherBodyIndex :type Integer) (bFromSweep :type Boolean) (SweepResult :type Hit%20Result%20Structure%20%28by%20ref%29))
  (if (Variables|Default|GetIsTrigger)
    (if (Variables|Default|GetPlatformDown)
      (CallFunction|PlatformGoUp)
      (else
        (CallFunction|PlatformGoDown)))))

(event OnComponentEndOverlap(Box)
  (params (OtherActor :type Actor%20Object%20Reference) (OtherComp :type Primitive%20Component%20Object%20Reference) (OtherBodyIndex :type Integer))
  (bind _moving_platform_with_trigger_ (Timeline|Moving%20Platform%20with%20Trigger Stop)
    (:Update
      (Transformation|SetRelativeLocation (Variables|Default|GetModel%20-%20MovingPlatform) (Math|Vector|Lerp(Vector) (Variables|Default|GetMovingPlatformStart) (Variables|Default|GetMovingPlatformEnd) _moving_platform_with_trigger_) false))))

(event Custom|Platform%20Go%20Down
  (Variables|Default|SetPlatformDown true)
  (bind _moving_platform_with_trigger_ (Timeline|Moving%20Platform%20with%20Trigger Reverse)
    (:Update
      (Transformation|SetRelativeLocation (Variables|Default|GetModel%20-%20MovingPlatform) (Math|Vector|Lerp(Vector) (Variables|Default|GetMovingPlatformStart) (Variables|Default|GetMovingPlatformEnd) _moving_platform_with_trigger_) false))))

(event Custom|Platform%20Go%20Up
  (Variables|Default|SetPlatformDown false)
  (bind _moving_platform_with_trigger_ (Timeline|Moving%20Platform%20with%20Trigger Play)
    (:Update
      (Transformation|SetRelativeLocation (Variables|Default|GetModel%20-%20MovingPlatform) (Math|Vector|Lerp(Vector) (Variables|Default|GetMovingPlatformStart) (Variables|Default|GetMovingPlatformEnd) _moving_platform_with_trigger_) false))))

(event EventBeginPlay
  (Rendering|Material|CreateDynamicMaterialInstance (Variables|Default|GetModel%20-%20MovingPlatform) 0 (Variables|Default|GetMaterial) :!class /Script/Engine.PrimitiveComponent)
  (if (not (Variables|Default|GetIsTrigger))
    (bind _moving_platform (Timeline|Moving%20Platform Play)
      (:Update
        (Transformation|SetRelativeLocation (Variables|Default|GetModel%20-%20MovingPlatform) (Math|Vector|Lerp(Vector) (Variables|Default|GetMovingPlatformStart) (Variables|Default|GetMovingPlatformEnd) _moving_platform) false)))))

(fn ConstructionScript)