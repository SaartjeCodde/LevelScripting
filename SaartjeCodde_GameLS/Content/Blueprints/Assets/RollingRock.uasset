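; RollingRock is an actor that gets pushed along and can drop into a hole.
; Each hit on the Rock component moves the actor without sweep along the player pawn's forward vector by Speed times delta time, whatever it collided with.
; The same hit adds a fixed roll step scaled by that vector's Y component.
; A separate FallDown event instantly offsets the actor downward to sink it into the hole.
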(event OnComponentHit(Rock)
  (params (OtherActor :type Actor%20Object%20Reference) (OtherComp :type Primitive%20Component%20Object%20Reference) (NormalImpulse :type Vector :default "0, 0, 0") (Hit :type Hit%20Result%20Structure%20%28by%20ref%29))
  (bind _rock (Variables|Default|GetRock))
  (bind _returnvalue (Transformation|GetWorldTransform _rock))
  (bind (_location _rotation _scale) (Math|Transform|BreakTransform _returnvalue))
  (Transformation|SetActorTransform (Math|Transform|MakeTransform (+ (* (Math|Vector|Normalize (Transformation|GetActorForwardVector (Game|Player|GetPlayerPawn 0))) (* (Utilities|Time|GetWorldDeltaSeconds) (Variables|Default|GetSpeed))) _location) _rotation _scale))
  (Transformation|AddActorLocalRotation (* (Class|KismetMathLibrary|MakeRot 0.0 0.0 2.0) (.Y (Math|Vector|BreakVector (Math|Vector|Normalize (Transformation|GetActorForwardVector (Game|Player|GetPlayerPawn 0)))))) false))

(event Custom|Fall%20Down!
  ;[1 1 1] Fall in hole
  (Transformation|AddActorLocalOffset "0, 0,-100.000000" false))

(fn ConstructionScript)